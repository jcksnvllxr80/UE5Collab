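; Player controller that runs the death sequence when OnDeath fires.
; It starts a slow camera fade to black, shows the WBP_YouDied widget, then after a short delay plays a random death voice line through a looping MultiGate.
; The widget is removed after a further delay, but the final game mode cast leads nowhere, as the restart and possession nodes are disconnected.
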(event `OnDeath`
  (`PlayerCameraManager.StartCameraFade` (`self.PlayerCameraManager`) 0.0 1.0 15.0 (struct :`A` 1.0) false true)
  (bind _returnvalue (`|CreateWidget` "/Game/import/Suburu/SuburuSkelMesh/WBP_YouDied.WBP_YouDied_C" self))
  (`UserWidget.AddToViewport` _returnvalue 0)
  (`KismetSystemLibrary.Delay` 1.0)
  (`|MultiGate` true true
    (:`Out 0`
      (`GameplayStatics.PlaySound2D` "/Game/import/Sounds/OnDeathNarration/Carcus.Carcus" 1.0 1.0 0.0 null null))
    (:`Out 1`
      (`GameplayStatics.PlaySound2D` "/Game/import/Sounds/OnDeathNarration/pitiful.pitiful" 1.0 1.0 0.0 null null))
    (:`Out 2`
      (`GameplayStatics.PlaySound2D` "/Game/import/Sounds/OnDeathNarration/WelcomeToYourDoom.WelcomeToYourDoom" 1.0 1.0 0.0 null null))
    (:`Out 3`
      (`GameplayStatics.PlaySound2D` "/Game/import/Sounds/OnDeathNarration/Carcus01.Carcus01" 1.0 1.0 0.0 null null))
    (:`Out 4`
      (`GameplayStatics.PlaySound2D` "/Game/import/Sounds/OnDeathNarration/YouDied.YouDied" 1.0 1.0 0.0 null null))
    (:`Out 5`
      (`GameplayStatics.PlaySound2D` "/Game/import/Sounds/OnDeathNarration/YourGraveAwaits.YourGraveAwaits" 1.0 1.0 0.0 null null))
    (:`Out 6`
      (`GameplayStatics.PlaySound2D` "/Game/import/Sounds/OnDeathNarration/YouGraveAwaitsYouHAHAHA.YouGraveAwaitsYouHAHAHA" 1.0 1.0 0.0 null null)))
  (`KismetSystemLibrary.Delay` 10.0)
  (`Widget.RemoveFromParent` _returnvalue)
  (bind _asthird_person_game_mode (cast `/Game/ThirdPersonBP/Blueprints/ThirdPersonGameMode` (`GameplayStatics.GetGameMode`))))

(fn `UserConstructionScript`)