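; NSX car Blueprint, by its name, with an early setup for rolling down the right window by input.
; Pressing Roll Right Window Down sets WindowR's relative Z and roll through FInterpTo toward a lowered, tilted target.
; The interpolation runs once per press with no delta time wired, so it does not animate the window.
; Left-window logic is unconnected, and the other events and function are disabled or empty.
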(event `InputAction|Roll Right Window Down`
  (params (Key :type "Key Structure"))
  (bind _windowr (`self.WindowR`))
  (bind _returnvalue (`SceneComponent.GetRelativeTransform` _windowr))
  ;[1 1 1] WindowRoll Down
  (:`Pressed`
    (`SceneComponent.K2_SetRelativeLocation` _windowr (`KismetMathLibrary.MakeVector` 0.0 0.0 (`KismetMathLibrary.FInterpTo` (.z (.location _returnvalue)) -25.0 0.0 1.0)) false false)
    (`SceneComponent.K2_SetRelativeRotation` _windowr (`KismetMathLibrary.MakeRotator` (`KismetMathLibrary.FInterpTo` (.roll (.rotation _returnvalue)) 15.0 0.0 1.0)) false false)))

(fn `NewFunction_0`)

(fn `UserConstructionScript`
  (`parent.UserConstructionScript`))