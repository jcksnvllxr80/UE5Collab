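; Drivable, armed Subaru pawn on Chaos vehicle physics, possessed through EnterCar, with machine guns, smoke, oil slick and flares.
; Inputs feed movement, gears, camera, sounds and time dilation, and switch lights through material swaps and intensity changes.
; Tick runs DriftDetect, which checks wheel slip on a skid surface to drive tire smoke and squeal.
; At zero health it explodes, swaps meshes, spawns debris and a ragdoll driver, and notifies BP_PlayerController.
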(event `InputAction|DomeLight`
  (params (Key :type "Key Structure"))
  (bind _domelight (`self.DomeLight`))
  ;[1 1 1] DomeLight
  (:`Pressed`
    (`/Engine/EditorBlueprintResources/StandardMacros.FlipFlop`
      (:`A`
        (`LightComponent.SetIntensity` _domelight 500.0)
        (`PrimitiveComponent.SetMaterial` (`self.DomeLightMesh`) 0 "/Game/AirCar/Glass_Head_light_.Glass_Head_light_"))
      (:`B`
        (`LightComponent.SetIntensity` _domelight 0.0)
        (`PrimitiveComponent.SetMaterial` (`self.DomeLightMesh`) 0 "/Game/import/Suburu/SuburuSkelMesh/HeadLightOffGlass1_Inst.HeadLightOffGlass1_Inst")))))

(event `Key|K`
  (params (Key :type "Key Structure"))
  (bind _mesh (`self.Mesh`))
  ;[1 1 1] Hazards Lights Test
  (:`Pressed`
    (`/Engine/EditorBlueprintResources/StandardMacros.FlipFlop`
      (:`A`
        (set `self.HazardsON` true)
        (`PrimitiveComponent.SetMaterial` _mesh 25 "/Game/AirCar/YellowLight.YellowLight" :!label _label)
        (`KismetSystemLibrary.Delay` 0.35)
        (`PrimitiveComponent.SetMaterial` _mesh 25 "/Game/import/Suburu/SuburuSkelMesh/YellowTintedGlassInst.YellowTintedGlassInst")
        (`KismetSystemLibrary.Delay` 0.35)
        (if (`self.HazardsON`)
          (goto _label)))
      (:`B`
        (set `self.HazardsON` false)
        (if (`self.HeadlightsActive`)
          (set `self.parkinglightson` true)
          (`PrimitiveComponent.SetMaterial` _mesh 25 "/Game/AirCar/YellowLight.YellowLight"))))))

(event `self.ReceiveTick`
  (params (DeltaSeconds :type "Float (single-precision)"))
  (bind _rl (`self.RL`))
  (bind _mesh (`self.Mesh`))
  (bind _relativerotation_roll (`KismetMathLibrary.BreakRotator` (`SceneComponent.RelativeRotation` (`self.Mesh`))))
  (`|ExecutionSequence`
    (:`then_0`
      (`self.DriftDetect`)
      ;[1 1 1] ReverseLight
      (`/Engine/EditorBlueprintResources/StandardMacros.CompareFloat` (`ChaosVehicleMovementComponent.GetForwardSpeed` (`self.Vehicle Movement Component`)) -1.0
        (:`>`
          (`PrimitiveComponent.SetMaterial` (`self.Mesh`) 4 "/Game/import/Suburu/SuburuSkelMesh/WhiteTintedGlass_Inst.WhiteTintedGlass_Inst"))
        (:`==`
          (set `self.Reversing` true :!label _label_2))
        (:`<`
          (goto _label_2)))
      (`LightComponent.SetIntensity` (`self.Reverse`) 0.0))
    (:`then_1`
      ;[1 1 1] Damage
      ;;[1 1 1] roll death - not working
      (if (== _relativerotation_roll 90.0)
        _))
    (:`then_2`
      (if (`self.parkinglightson`)
        (`PrimitiveComponent.SetMaterial` _mesh 25 "/Game/AirCar/YellowLight.YellowLight")
        (else
          (`PrimitiveComponent.SetMaterial` _mesh 25 "/Game/import/Suburu/SuburuSkelMesh/YellowTintedGlassInst.YellowTintedGlassInst"))))
    (:`then_3`
      ;[1 1 1] DriftingTireSmoke
      (if (`self.Drifting`)
        (`ActorComponent.Activate` _rl false)
        (`ActorComponent.Activate` (`self.FR`) false)
        (`ActorComponent.Activate` (`self.RR`) false)
        (`ActorComponent.Activate` (`self.FLtiresmoke`) false)
        (else
          (`ActorComponent.Deactivate` _rl)
          (`ActorComponent.Deactivate` (`self.RR`))
          (`ActorComponent.Deactivate` (`self.FLtiresmoke`))
          (`ActorComponent.Deactivate` (`self.FR`)))))))

(event `InputAction|HeadLightKnob`
  (params (Key :type "Key Structure"))
  (bind _headlightr (`self.HeadLightR`))
  (bind _mesh (`self.Mesh`))
  ;[1 1 1] Headlight Code
  (:`Pressed`
    (`|MultiGate` false true
      (:`Out 0`
        (set `self.parkinglightson` (`self.parkinglightson`))
        (if (not (`self.HazardsON`))
          ;;[1 1 1] bypass yellowlights
          (`PrimitiveComponent.SetMaterial` _mesh 25 "/Game/AirCar/YellowLight.YellowLight"))
        (`PrimitiveComponent.SetMaterial` _mesh 6 "/Game/import/Suburu/SuburuSkelMesh/BrakeLight1_Inst.BrakeLight1_Inst")
        (`LightComponent.SetIntensity` (`self.BrakeR`) 2500.0)
        (`LightComponent.SetIntensity` (`self.BrakeL`) 2500.0)
        (set `self.HeadlightsActive` true))
      (:`Out 1`
        (`LightComponent.SetIntensity` _headlightr 50000.0)
        (`LightComponent.SetIntensity` (`self.HeadLightL`) 50000.0)
        (`PrimitiveComponent.SetMaterial` (`self.Mesh`) 17 "/Game/AirCar/Glass_Head_light_.Glass_Head_light_"))
      (:`Out 2`
        (`LightComponent.SetIntensity` _headlightr 150000.0)
        (`LightComponent.SetIntensity` (`self.HeadLightL`) 150000.0))
      (:`Out 3`
        (if (not (`self.HazardsON`))
          (`PrimitiveComponent.SetMaterial` _mesh 25 "/Game/import/Suburu/SuburuSkelMesh/YellowTintedGlassInst.YellowTintedGlassInst"))
        (`LightComponent.SetIntensity` _headlightr 0.0)
        (`LightComponent.SetIntensity` (`self.HeadLightL`) 0.0)
        (`LightComponent.SetIntensity` (`self.BrakeL`) 0.0)
        (`LightComponent.SetIntensity` (`self.BrakeR`) 0.0)
        (`PrimitiveComponent.SetMaterial` _mesh 17 "/Game/import/Materials/GlassReflection.GlassReflection")
        (`PrimitiveComponent.SetMaterial` _mesh 6 "/Game/import/Suburu/SuburuSkelMesh/TintedGlass_Inst.TintedGlass_Inst")
        (set `self.HeadlightsActive` false)))))

(event `self.ReceiveBeginPlay`
  ;[1 1 1] Comment
  (bind _aschaos_wheeled_vehicle_movement_component (cast `ChaosWheeledVehicleMovementComponent` (`self.VehicleMovementComponent`)))
  (set `self.Vehicle Movement Component` _aschaos_wheeled_vehicle_movement_component))

(event `Key|Zero`
  (params (Key :type "Key Structure"))
  (:`Pressed`
    (`PrimitiveComponent.SetConstraintMode` (`self.Mesh`) "None")))

(event `InputAxis|Throttle`
  (params (AxisValue :type "Float (single-precision)"))
  ;[1 1 1] Car Basic Controls
  (`ChaosVehicleMovementComponent.SetThrottleInput` (`self.VehicleMovementComponent`) AxisValue)
  (`/Engine/EditorBlueprintResources/StandardMacros.CompareFloat` AxisValue -1.0))

(event `InputAxis|Brake`
  (params (AxisValue :type "Float (single-precision)"))
  ;[1 1 1] Car Basic Controls
  (`ChaosVehicleMovementComponent.SetBrakeInput` (`self.VehicleMovementComponent`) AxisValue))

(event `InputAction|Horn`
  (params (Key :type "Key Structure"))
  ;[1 1 1] Horn
  (:`Pressed`
    (`GameplayStatics.SpawnSoundAttached` "/Game/import/Suburu/horn.horn" (`self.Mesh`) "None" (0.0 0.0 0.0) (struct) "KeepRelativeOffset" false 1.0 1.0 0.0 null null)))

(event `InputAxis|Steering`
  (params (AxisValue :type "Float (single-precision)"))
  ;[1 1 1] Car Basic Controls
  (`ChaosVehicleMovementComponent.SetSteeringInput` (`self.VehicleMovementComponent`) AxisValue))

(event `InputAction|HandBrake`
  (params (Key :type "Key Structure"))
  (bind _vehiclemovementcomponent (`self.VehicleMovementComponent`))
  ;[1 1 1] Car Basic Controls
  (:`Pressed`
    (`ChaosVehicleMovementComponent.SetHandbrakeInput` _vehiclemovementcomponent true))
  (:`Released`
    (`ChaosVehicleMovementComponent.SetHandbrakeInput` _vehiclemovementcomponent false)))

(event `Key|S`
  (params (Key :type "Key Structure"))
  (bind _mesh (`self.Mesh`))
  (bind _headlightsactive (`self.HeadlightsActive`))
  (bind _braker (`self.BrakeR`))
  ;[1 1 1] BrakeLights - Variable "HeadlightsActive" reroutes released brake lights to keep at 5000 intensity when headlights are on. "Set Material" element changes brake light lens from see through glass to red colored emmissive (glowing) material
  (:`Pressed`
    (if _headlightsactive
      (`PrimitiveComponent.SetMaterial` _mesh 6 "/Game/import/Suburu/SuburuSkelMesh/TintedGlass_Inst.TintedGlass_Inst" :!label _label_3)
      (`LightComponent.SetIntensity` _braker 0.0)
      (`LightComponent.SetIntensity` (`self.BrakeL`) 0.0)
      (else
        (`PrimitiveComponent.SetMaterial` _mesh 6 "/Game/import/Suburu/SuburuSkelMesh/BrakeLightHigh.BrakeLightHigh")
        (`LightComponent.SetIntensity` _braker 5000.0)
        (`LightComponent.SetIntensity` (`self.BrakeL`) 5000.0))))
  (:`Released`
    (if _headlightsactive
      (`LightComponent.SetIntensity` _braker 2500.0)
      (`LightComponent.SetIntensity` (`self.BrakeL`) 2500.0)
      (else
        (goto _label_3)))))

(event `InputAxisKey|MouseWheelAxis`
  (params (AxisValue :type "Float (single-precision)"))
  ;[1 1 1] Camera Zoom
  (`SceneComponent.K2_AddRelativeLocation` (`self.Camera`) (`KismetMathLibrary.MakeVector` (* AxisValue 40.0)) false false))

(event `InputAxisKey|MouseX`
  (params (AxisValue :type "Float (single-precision)"))
  ;[1 1 1] MouseLook
  (`SceneComponent.K2_AddRelativeRotation` (`self.SpringArm`) (`KismetMathLibrary.MakeRotator` 0.0 0.0 (* AxisValue 2.0)) false false))

(event `InputAction|Taunt`
  (params (Key :type "Key Structure"))
  (bind _mesh (`self.Mesh`))
  ;[1 1 1] Taunt
  (:`Pressed`
    (`|MultiGate` true true
      (:`Out 0`
        (`GameplayStatics.SpawnSoundAttached` "/Game/import/Suburu/surprise.surprise" _mesh "None" (0.0 0.0 0.0) (struct) "KeepRelativeOffset" false 1.0 1.0 0.0 null null))
      (:`Out 1`
        (`GameplayStatics.SpawnSoundAttached` "/Game/import/Suburu/GetThatCornOuttaMyFace.GetThatCornOuttaMyFace" _mesh "None" (0.0 0.0 0.0) (struct) "KeepRelativeOffset" false 1.0 1.0 0.0 null null))
      (:`Out 2`
        (`GameplayStatics.SpawnSoundAttached` "/Game/import/Suburu/SaveCorn.SaveCorn" _mesh "None" (0.0 0.0 0.0) (struct) "KeepRelativeOffset" false 1.0 1.0 0.0 null null))
      (:`Out 3`
        (`GameplayStatics.SpawnSoundAttached` "/Game/import/Suburu/Ahh.Ahh" _mesh "None" (0.0 0.0 0.0) (struct) "KeepRelativeOffset" false 1.0 1.0 0.0 null null)))))

(event `InputAxisKey|MouseY`
  (params (AxisValue :type "Float (single-precision)"))
  ;[1 1 1] MouseLook
  (`SceneComponent.K2_AddRelativeRotation` (`self.SpringArm`) (`KismetMathLibrary.MakeRotator` 0.0 (* AxisValue 2.0)) false false))

(event `Key|BackSpace`
  (params (Key :type "Key Structure"))
  ;[1 1 1] Rollover Code
  (:`Pressed`
    (`self.K2_TeleportTo` (`GameplayStatics.GetPlayerPawn` 0) (0.0 0.0 10.0) (struct :`Roll` 90.0))))

(event `InputAction|HandBrake`
  (params (Key :type "Key Structure"))
  (bind _braker (`self.BrakeR`))
  (bind _mesh (`self.Mesh`))
  ;[1 1 1] handbrake
  (:`Pressed`
    (`PrimitiveComponent.SetMaterial` _mesh 6 "/Game/import/Suburu/SuburuSkelMesh/BrakeLightHigh.BrakeLightHigh")
    (`LightComponent.SetIntensity` _braker 5000.0)
    (`LightComponent.SetIntensity` (`self.BrakeL`) 5000.0))
  (:`Released`
    (if (`self.HeadlightsActive`)
      (`LightComponent.SetIntensity` _braker 2500.0)
      (`LightComponent.SetIntensity` (`self.BrakeL`) 2500.0)
      (else
        (`PrimitiveComponent.SetMaterial` _mesh 6 "/Game/import/Suburu/SuburuSkelMesh/TintedGlass_Inst.TintedGlass_Inst")
        (`LightComponent.SetIntensity` _braker 0.0)
        (`LightComponent.SetIntensity` (`self.BrakeL`) 0.0)))))

(event `Key|E`
  (params (Key :type "Key Structure"))
  ;[1 1 1] Gear Test Code
)

(event `Key|Q`
  (params (Key :type "Key Structure"))
  ;[1 1 1] Gear Test Code
)

(event `Key|One`
  (params (Key :type "Key Structure"))
  ;[1 1 1] Gear Test Code
  (:`Pressed`
    (`ChaosVehicleMovementComponent.SetTargetGear` (`self.VehicleMovementComponent`) 1 true)))

(event `/Game/Blueprints/BPI_DamageInterface.TakeDamage`
  (params (Damage :type "Float (double-precision)"))
  (bind _destroyedmesh (`self.DestroyedMesh`))
  (bind _mesh (`self.Mesh`))
  (bind (_returnvalue_location _returnvalue_rotation) (`KismetMathLibrary.BreakTransform` (`SceneComponent.K2_GetComponentToWorld` _mesh)))
  (bind (_returnvalue_location_2 _returnvalue_rotation_2) (`KismetMathLibrary.BreakTransform` (`SceneComponent.K2_GetComponentToWorld` (`self.Manarrow`))))
  (bind (_returnvalue_location_3 _returnvalue_rotation_3) (`KismetMathLibrary.BreakTransform` (`SceneComponent.K2_GetComponentToWorld` (`self.explopush`))))
  (bind _returnvalue (`SceneComponent.K2_GetComponentLocation` _mesh))
  (bind _returnvalue_2 (`KismetMathLibrary.Conv_VectorToTransform` _returnvalue))
  (bind _returnvalue_3 (`KismetMathLibrary.Conv_VectorToTransform` _returnvalue))
  (bind _returnvalue_4 (+ _returnvalue (0.0 0.0 90.0)))
  ;[1 1 1] Damage
  (bind _output_get (set `self.Health` (- (`self.Health`) Damage)))
  (`KismetSystemLibrary.PrintString` (`KismetStringLibrary.Conv_DoubleToString` _output_get))
  (if (<= _output_get 0.0)
    (`GameplayStatics.PlaySoundAtLocation` "/Game/StarterContent/Audio/Explosion02.Explosion02" _returnvalue (struct) 1.0 1.0 0.0 null null null null)
    (`NiagaraFunctionLibrary.SpawnSystemAtLocation` null (+ _returnvalue (100.0 0.0 25.0)) _returnvalue_rotation (2.0 2.0 2.0))
    (`GameplayStatics.SpawnEmitterAtLocation` "/Game/MyParticleSystems/Sprite/P_SparksZeroG1.P_SparksZeroG1" _returnvalue_4 (struct :`Pitch` 90.0) (0.75 0.75 0.75))
    (`GameplayStatics.SpawnEmitterAttached` "/Game/StarterContent/Particles/P_Fire1.P_Fire1" _destroyedmesh "None" (0.0 0.0 50.0))
    (`GameplayStatics.SpawnEmitterAttached` "/Game/StarterContent/Particles/P_Fire1.P_Fire1" _destroyedmesh "None")
    (`SceneComponent.ToggleVisibility` (`self.Mesh`) true)
    (`SceneComponent.ToggleVisibility` (`self.DestroyedMesh`) true)
    ;[1 1 1] DesTires
    (bind _returnvalue_5 (`|SpawnActorFromClass` "/Game/Blueprints/DestroyedActors/TrunkDestroyed.TrunkDestroyed_C" _returnvalue_3 "AlwaysSpawn" "OverrideRootScale" null null))
    (bind _returnvalue_6 (`|SpawnActorFromClass` "/Game/Blueprints/DestroyedActors/Tires/FRTireDes.FRTireDes_C" _returnvalue_3 "AlwaysSpawn" "OverrideRootScale" null null))
    (bind _returnvalue_7 (`|SpawnActorFromClass` "/Game/Blueprints/DestroyedActors/Tires/LRTireDes.LRTireDes_C" _returnvalue_3 "AlwaysSpawn" "OverrideRootScale" null null))
    (bind _returnvalue_8 (`|SpawnActorFromClass` "/Game/Blueprints/DestroyedActors/Tires/RRTireDes.RRTireDes_C" _returnvalue_3 "AlwaysSpawn" "OverrideRootScale" null null))
    (`|SpawnActorFromClass` "/Game/Blueprints/DestroyedActors/HoodDestroyed.HoodDestroyed_C" _returnvalue_3 "AlwaysSpawn" "OverrideRootScale" null null)
    (`|SpawnActorFromClass` "/Game/Blueprints/DestroyedActors/Tires/FLTireDes.FLTireDes_C" _returnvalue_3 "AlwaysSpawn" "OverrideRootScale" null null)
    (`|SpawnActorFromClass` "/Game/Blueprints/DestroyedActors/FLDoorDes.FLDoorDes_C" _returnvalue_3 "AlwaysSpawn" "OverrideRootScale" null null)
    (`|SpawnActorFromClass` "/Game/Blueprints/DestroyedActors/FRDoorDes.FRDoorDes_C" (`KismetMathLibrary.MakeTransform` _returnvalue_4) "AlwaysSpawn" "OverrideRootScale" null null)
    (`|SpawnActorFromClass` "/Game/Blueprints/DestroyedActors/DesEngine.DesEngine_C" (`KismetMathLibrary.Conv_VectorToTransform` (+ _returnvalue (100.0 0.0 90.0))) "AlwaysSpawn" "OverrideRootScale" null null)
    (`|SpawnActorFromClass` "/Game/Blueprints/DestroyedActors/DesTrans.DesTrans_C" (`KismetMathLibrary.Conv_VectorToTransform` (+ _returnvalue (0.0 0.0 12.0))) "AlwaysSpawn" "OverrideRootScale" null null)
    (`|SpawnActorFromClass` "/Game/Blueprints/DestroyedActors/DesRightDoor.DesRightDoor_C" _returnvalue_2 "AlwaysSpawn" "OverrideRootScale" null null)
    (`|SpawnActorFromClass` "/Game/Blueprints/DestroyedActors/DesRightRearDoor.DesRightRearDoor_C" _returnvalue_2 "AlwaysSpawn" "OverrideRootScale" null null)
    (`|SpawnActorFromClass` "/Game/Blueprints/DestroyedActors/DesSteeringWheel.DesSteeringWheel_C" (`KismetMathLibrary.MakeTransform` _returnvalue) "AlwaysSpawn" "OverrideRootScale" null null)
    (`|SpawnActorFromClass` "/Game/Blueprints/DestroyedActors/DesCarSeat.DesCarSeat_C" (`KismetMathLibrary.MakeTransform` _returnvalue) "AlwaysSpawn" "OverrideRootScale" null null)
    ;;[1 1 1] Cheat to Induce Explo-velocity
    (`|SpawnActorFromClass` "/Game/Blueprints/explopush.explopush_C" (`KismetMathLibrary.MakeTransform` _returnvalue_location_3 _returnvalue_rotation_3) "Undefined" "OverrideRootScale" null null)
    (`KismetSystemLibrary.Delay` 0.05)
    (bind _returnvalue_9 (`|SpawnActorFromClass` "/Game/Blueprints/DestroyedActors/DeadDriver.DeadDriver_C" (`KismetMathLibrary.MakeTransform` (+ _returnvalue_location_2 (0.0 0.0 0.0)) _returnvalue_rotation_2) "AdjustIfPossibleButAlwaysSpawn" "OverrideRootScale" null null))
    (`SkeletalMeshComponent.SetAllBodiesSimulatePhysics` (`/Game/Blueprints/DestroyedActors/DeadDriver.SkeletalMesh` _returnvalue_9) true)
    (bind _asbp_player_controller (cast `/Game/Blueprints/BP_PlayerController` (`self.GetController`)))
    (`PrimitiveComponent.SetSimulatePhysics` (`self.FixerCube`) true)
    (`/Game/Blueprints/BP_PlayerController.OnDeath` _asbp_player_controller)))

(event `Key|Two`
  (params (Key :type "Key Structure"))
  ;[1 1 1] Gear Test Code
  (:`Pressed`
    (`ChaosVehicleMovementComponent.SetTargetGear` (`self.VehicleMovementComponent`) 2 true)))

(event `Key|Three`
  (params (Key :type "Key Structure"))
  ;[1 1 1] Gear Test Code
  (:`Pressed`
    (`ChaosVehicleMovementComponent.SetTargetGear` (`self.VehicleMovementComponent`) 3 true)))

(event `Key|Four`
  (params (Key :type "Key Structure"))
  ;[1 1 1] Gear Test Code
  (:`Pressed`
    (`ChaosVehicleMovementComponent.SetTargetGear` (`self.VehicleMovementComponent`) 4 true)))

(event `Key|Five`
  (params (Key :type "Key Structure"))
  ;[1 1 1] Gear Test Code
  (:`Pressed`
    (`ChaosVehicleMovementComponent.SetTargetGear` (`self.VehicleMovementComponent`) 5 true)))

(event `Key|Six`
  (params (Key :type "Key Structure"))
  ;[1 1 1] Gear Test Code
  (:`Pressed`
    (`ChaosVehicleMovementComponent.SetTargetGear` (`self.VehicleMovementComponent`) 6 true)))

(event `Key|R`
  (params (Key :type "Key Structure"))
  ;[1 1 1] Gear Test Code
  (:`Pressed`
    (`ChaosVehicleMovementComponent.SetTargetGear` (`self.VehicleMovementComponent`) -1 false)))

(event `Key|T`
  (params (Key :type "Key Structure"))
  ;[1 1 1] time dilation - SLOW
  (:`Pressed`
    (`/Engine/EditorBlueprintResources/StandardMacros.FlipFlop`
      (:`A`
        (`GameplayStatics.SetGlobalTimeDilation` 0.25))
      (:`B`
        (`GameplayStatics.SetGlobalTimeDilation` 1.0)))
    (set `Actor.CustomTimeDilation` 1.0 (`GameplayStatics.GetPlayerCharacter` 0))))

(event `self.Box.OnComponentBeginOverlap`
  (params (OverlappedComponent :type "PrimitiveComponent Object Reference") (OtherActor :type "Actor Object Reference") (OtherComp :type "PrimitiveComponent Object Reference") (OtherBodyIndex :type Integer) (bFromSweep :type Boolean) (SweepResult :type "HitResult Structure (by ref)"))
  ;[1 1 1] PawnSwitch
  (bind _asthird_person_character (cast `/Game/ThirdPersonBP/Blueprints/ThirdPersonCharacter` OtherActor))
  (set `/Game/ThirdPersonBP/Blueprints/ThirdPersonCharacter.Near Car?` true _asthird_person_character))

(event `self.Box.OnComponentEndOverlap`
  (params (OverlappedComponent :type "PrimitiveComponent Object Reference") (OtherActor :type "Actor Object Reference") (OtherComp :type "PrimitiveComponent Object Reference") (OtherBodyIndex :type Integer))
  ;[1 1 1] PawnSwitch
  (bind _asthird_person_character (cast `/Game/ThirdPersonBP/Blueprints/ThirdPersonCharacter` OtherActor)))

(event `Key|Shift+T`
  (params (Key :type "Key Structure"))
  ;[1 1 1] Time Freeze
  (:`Pressed`
    (`/Engine/EditorBlueprintResources/StandardMacros.FlipFlop`
      (:`A`
        (`GameplayStatics.SetGlobalTimeDilation` 0.0))
      (:`B`
        (`GameplayStatics.SetGlobalTimeDilation` 1.0)))
    (set `Actor.CustomTimeDilation` 1.0 (`GameplayStatics.GetPlayerCharacter` 0))))

(event `Enter Car`
  ;[1 1 1] PawnSwitch
  (`Controller.Possess` (`GameplayStatics.GetPlayerController` 0) self)
  (set `self.DrivingCar?` true))

(event `Key|Divide`
  (params (Key :type "Key Structure"))
  ;[1 1 1] not working car reset
  (:`Pressed`
    (`ChaosVehicleMovementComponent.ResetVehicle` (`self.VehicleMovementComponent`))))

(event `self.PawnSensing.OnSeePawn`
  (params (Pawn :type "Pawn Object Reference"))
  ;[1 1 1] AI test
  (bind _asbp_suburu (cast `/Game/Blueprints/BP_Suburu` Pawn))
  (bind (_returnvalue_location _returnvalue_rotation) (`KismetMathLibrary.BreakTransform` (`SceneComponent.K2_GetComponentToWorld` (`Actor.RootComponent` _asbp_suburu))))
  (`KismetSystemLibrary.MoveComponentTo` null _returnvalue_location _returnvalue_rotation))

(event `Key|Comma`
  (params (Key :type "Key Structure"))
  (bind (_returnvalue_location _returnvalue_rotation) (`KismetMathLibrary.BreakTransform` (`SceneComponent.K2_GetComponentToWorld` (`self.SmokeAttached`))))
  ;[1 1 1] smokedeploy
  (:`Pressed`
    (`|SpawnActorFromClass` "/Game/Blueprints/SmokeCanisters.SmokeCanisters_C" (`KismetMathLibrary.MakeTransform` (+ _returnvalue_location (0.0 0.0 20.0)) _returnvalue_rotation (0.075 0.075 0.075)) "AdjustIfPossibleButAlwaysSpawn" "OverrideRootScale" self null)))

(event `Key|Period`
  (params (Key :type "Key Structure"))
  ;[1 1 1] oilslick
  (:`Pressed`
    (`/Engine/EditorBlueprintResources/StandardMacros.FlipFlop`
      (:`A`
        (`ActorComponent.Activate` (`self.OilParticle`) false))
      (:`B`
        (`ActorComponent.Deactivate` (`self.OilParticle`))))))

(event `Key|LeftControl`
  (params (Key :type "Key Structure"))
  (bind _muzzleflash1 (`self.MuzzleFlash1`))
  (bind _muzzleflash2 (`self.MuzzleFlash2`))
  ;[1 1 1] Guns
  (:`Pressed`
    (set `self.IsFiring` true)
    (`|ExecutionSequence` :!label _label_4
      (:`then_0`
        (`|MultiGate` false true
          (:`Out 0`
            (`KismetSystemLibrary.Delay` 0.01)
            (`|SpawnActorFromClass` "/Game/Blueprints/TracerRound.TracerRound_C" (`SceneComponent.K2_GetComponentToWorld` (`self.GunBarrel`)) "Undefined" "OverrideRootScale" null null)
            (`SceneComponent.ToggleVisibility` _muzzleflash1 false)
            (`SceneComponent.ToggleVisibility` (`self.MF2b1`) false)
            (`GameplayStatics.PlaySoundAtLocation` "/Game/import/Suburu/SingleShotM60.SingleShotM60" (`SceneComponent.K2_GetComponentLocation` (`self.MachineGun1`)) (struct) 1.0 1.0 0.0 null null null null)
            (`KismetSystemLibrary.Delay` 0.05)
            (`SceneComponent.ToggleVisibility` _muzzleflash1 false)
            (`SceneComponent.ToggleVisibility` (`self.MF2b1`) false))
          (:`Out 1`
            (`KismetSystemLibrary.Delay` 0.01)
            (`|SpawnActorFromClass` "/Game/Blueprints/TracerRound.TracerRound_C" (`SceneComponent.K2_GetComponentToWorld` (`self.GunBarrel1`)) "Undefined" "OverrideRootScale" null null)
            (`SceneComponent.ToggleVisibility` _muzzleflash2 false)
            (`SceneComponent.ToggleVisibility` (`self.MF2b`) false)
            (`GameplayStatics.PlaySoundAtLocation` "/Game/import/Suburu/SingleShotM60.SingleShotM60" (`SceneComponent.K2_GetComponentLocation` (`self.Machinegun2`)) (struct) 1.0 1.0 0.0 null null null null)
            (`KismetSystemLibrary.Delay` 0.05)
            (`SceneComponent.ToggleVisibility` _muzzleflash2 false)
            (`SceneComponent.ToggleVisibility` (`self.MF2b`) false)))
        (if (`self.IsFiring`)
          (goto _label_4)
          (else
            (`SceneComponent.SetVisibility` (`self.MF2b1`) false false :!label _label_5)
            (`SceneComponent.SetVisibility` _muzzleflash1 false false)
            (`SceneComponent.SetVisibility` _muzzleflash2 false false)
            (`SceneComponent.SetVisibility` (`self.MF2b`) false false))))))
  (:`Released`
    (set `self.IsFiring` false)
    (goto _label_5)))

(event `Key|LeftAlt`
  (params (Key :type "Key Structure"))
  (bind _returnvalue_location (`KismetMathLibrary.BreakTransform` (`SceneComponent.K2_GetComponentToWorld` (`self.FlareOut`))))
  ;[1 1 1] Guns
  (:`Pressed`
    (`|SpawnActorFromClass` "/Game/Blueprints/Flare.Flare_C" (`KismetMathLibrary.MakeTransform` (+ _returnvalue_location (-50.0 0.0 0.0)) (struct :`Pitch` 100.0)) "Undefined" "OverrideRootScale" null null)))

(fn `BreakMesh`
  ;[1 1 1] doesnt work yet
)

(fn `DriftDetect`
  (bind _vehicle_movement_component (`self.Vehicle Movement Component`))
  (for (_ _array_index) (`ChaosWheeledVehicleMovementComponent.Wheels` _vehicle_movement_component)
    (bind (_bincontact _contactpoint _physmaterial _normalizedsuspensionlength _springforce _slipangle _bisslipping _slipmagnitude _bisskidding _skidmagnitude) (`ChaosWheeledVehicleMovementComponent.BreakWheelStatus` (`ChaosWheeledVehicleMovementComponent.GetWheelState` _vehicle_movement_component _array_index)))
    (if (and (== _physmaterial "/Game/import/Suburu/SuburuSkelMesh/SkidPhyMat.SkidPhyMat") (or (not (`KismetMathLibrary.NearlyEqual_FloatFloat` _slipmagnitude 0.0 0.1)) (not (`KismetMathLibrary.NearlyEqual_FloatFloat` _skidmagnitude 0.0 250.0))))
      (bind _returnvalue (select `int` _array_index :`0` (`self.NiagaraWheelParticleRL`) :`1` (`self.NiagaraWheelParticleRR`) :`2` (`self.NiagaraWheelParticleFR`) :`3` (`self.NiagaraWheelParticleFL`)))
      (`ActorComponent.Activate` _returnvalue false)
      (set `self.Drifting` true)
      (`GameplayStatics.PlaySoundAtLocation` "/Game/import/Suburu/TireSqueal.TireSqueal" (`SceneComponent.K2_GetComponentLocation` (`self.Mesh`)) (struct) 1.0 1.0 0.0 null null null null)
      (elif (`ActorComponent.IsActive` _returnvalue)
        (`ActorComponent.Deactivate` _returnvalue)
        (set `self.Drifting` false)))))

(fn `OIlSlick`
  (if (`self.OilSlicking`)
    (`ActorComponent.Activate` (`self.OilParticle`) false)
    (set `self.OilSlicking` true)
    (else
      (`ActorComponent.Deactivate` (`self.OilParticle`))
      (set `self.OilSlicking` false))))

(fn `OnRep_HeadlightsActive`)

(fn `UserConstructionScript`)