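; BP_Missile is a missile actor that destroys itself on overlap, with effects and player damage.
; An actor overlap spawns a collision sparks system at Sphere1 and sends a fixed damage message to player controller 0, without checking what it hit.
; A separate Sphere1 component overlap spawns a scaled-up explosion emitter and destroys the missile without sending damage.
; The graph contains no movement logic.
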(event `self.ReceiveActorBeginOverlap`
  (params (OtherActor :type "Actor Object Reference"))
  (bind (_returnvalue_location _returnvalue_rotation) (`KismetMathLibrary.BreakTransform` (`SceneComponent.K2_GetComponentToWorld` (`self.Sphere1`))))
  (`NiagaraFunctionLibrary.SpawnSystemAtLocation` "/Game/import/Suburu/SuburuSkelMesh/Particles/CollisionSparks_System.CollisionSparks_System" _returnvalue_location)
  (message `/Game/Blueprints/BPI_DamageInterface.TakeDamage` (`GameplayStatics.GetPlayerController` 0) 10.0)
  (`self.K2_DestroyActor`))

(event `self.Sphere1.OnComponentBeginOverlap`
  (params (OverlappedComponent :type "PrimitiveComponent Object Reference") (OtherActor :type "Actor Object Reference") (OtherComp :type "PrimitiveComponent Object Reference") (OtherBodyIndex :type Integer) (bFromSweep :type Boolean) (SweepResult :type "HitResult Structure (by ref)"))
  ;[1 1 1] missile explode
  (`GameplayStatics.SpawnEmitterAtLocation` "/Game/StarterContent/Particles/P_Explosion.P_Explosion" (`SceneComponent.K2_GetComponentLocation` (`self.Sphere1`)) (struct) (10.0 10.0 10.0))
  (`self.K2_DestroyActor`))

(fn `UserConstructionScript`)